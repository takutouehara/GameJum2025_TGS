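; BP_EnhancedInputTest is a test Blueprint that exercises Enhanced Input by printing input events to the screen.
; On BeginPlay it enables input from player 0 and adds IMC_Default to the Enhanced Input subsystem.
; IA_ActionA and IA_ActionB use DoOnce, reset on Completed, to print once per press and again on release.
; IA_Axis prints its X and Y values whenever it triggers.
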(event `self.ReceiveBeginPlay`
  (bind _returnvalue (`GameplayStatics.GetPlayerController` 0))
  (bind _returnvalue_2 (pcsubsystem `EnhancedInputLocalPlayerSubsystem` _returnvalue))
  (`|ExecutionSequence`
    (:`then_0`
      ;[1 1 1] 入力を有効にする
      (`self.EnableInput` _returnvalue))
    (:`then_1`
      ;[1 1 1] Input Mapping Contextを[IMC_Default]に設定する
      (`/Engine/EditorBlueprintResources/StandardMacros.IsValid` _returnvalue_2
        (:`Is Valid`
          (`EnhancedInputSubsystemInterface.AddMappingContext` _returnvalue_2 "/Game/Input/IMC_Default.IMC_Default" 0 (struct)))))))

(event `EnhancedInput|/Game/Input/Action/IA_ActionA`
  (params (ActionValue :type Boolean) (ElapsedSeconds :type "Float (double-precision)") (TriggeredSeconds :type "Float (double-precision)") (InputAction :type "InputAction Object Reference" :default "/Game/Input/Action/IA_ActionA.IA_ActionA"))
  ;[1 1 1] Action Input A
  (:`Triggered`
    (`/Engine/EditorBlueprintResources/StandardMacros.DoOnce` false :!label _label
      (:`Completed`
        (`KismetSystemLibrary.PrintString` "APressed"))))
  (:`Completed`
    (`|ExecutionSequence`
      (:`then_0`
        (goto _label :!via `Reset`))
      (:`then_1`
        (`KismetSystemLibrary.PrintString` "Released")))))

(event `EnhancedInput|/Game/Input/Action/IA_Axis`
  (params (ActionValue :type "Vector2D Structure") (ElapsedSeconds :type "Float (double-precision)") (TriggeredSeconds :type "Float (double-precision)") (InputAction :type "InputAction Object Reference" :default "/Game/Input/Action/IA_Axis.IA_Axis"))
  (bind (_x _y) (`KismetMathLibrary.BreakVector2D` ActionValue))
  ;[1 1 1] Axis（軸） Input
  (:`Triggered`
    (`KismetSystemLibrary.PrintString` (`KismetStringLibrary.Concat_StrStr` "X : " (`KismetStringLibrary.Conv_DoubleToString` _x) " Y : " (`KismetStringLibrary.Conv_DoubleToString` _y)))))

(event `EnhancedInput|/Game/Input/Action/IA_ActionB`
  (params (ActionValue :type Boolean) (ElapsedSeconds :type "Float (double-precision)") (TriggeredSeconds :type "Float (double-precision)") (InputAction :type "InputAction Object Reference" :default "/Game/Input/Action/IA_ActionB.IA_ActionB"))
  ;[1 1 1] Action Input B
  (:`Triggered`
    (`/Engine/EditorBlueprintResources/StandardMacros.DoOnce` false :!label _label_2
      (:`Completed`
        (`KismetSystemLibrary.PrintString` "BPressed"))))
  (:`Completed`
    (`|ExecutionSequence`
      (:`then_0`
        (goto _label_2 :!via `Reset`))
      (:`then_1`
        (`KismetSystemLibrary.PrintString` "Released")))))

(fn `UserConstructionScript`)
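; View-target camera actor that takes over player 0's view on BeginPlay, starting at the first camera in LevelCameras.
; SwitchCamera moves it toward the indexed level camera, using a timeline to lerp transform and FOV rather than changing view targets.
; The nodes that store the previous transform and FOV are disconnected, so the blend's start values are never updated here.
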(event `self.ReceiveBeginPlay`
  (bind (_returnvalue _field_of_view) (`self.GetCameraPosition ` 0))
  (`PlayerController.SetViewTargetWithBlend` (`GameplayStatics.GetPlayerController` 0) self 0.0 "VTBlend_Linear" 0.0 false)
  (`self.SetCameraPosition ` _returnvalue _field_of_view))

(event `/Game/EnhancedInput/Blueprints/BPI_SwitchCamera.SwitchCamera `
  (params (Index :type Integer))
  (bind (_returnvalue _field_of_view) (`self.GetCameraPosition ` Index))
  ;[1 1 1] New
  (set `self.NextTransform` _returnvalue)
  (set `self.NextFOV` _field_of_view)
  (set `self.Currenlndex` Index)
  (bind (_direction `_新規track_0`) (`Timeline|タイムライン` :!via `PlayFromStart`)
    (:`Update`
      (`self.SetCameraPosition ` (`KismetMathLibrary.TLerp` (`self.PreviousTransform`) (`self.NextTransform`) `_新規track_0`) (`KismetMathLibrary.Lerp` (`self.PreviousFOV`) (`self.NextFOV`) `_新規track_0`)))))

(fn `GetCameraPosition `
  (params (Index :type Integer))
  (returns (ReturnValue :type "Transform Structure (by ref)") (`Field Of View` :type "Float (single-precision)"))
  (bind _output (`|GetArrayItem` (`self.LevelCameras`) Index))
  (return (`self.GetTransform` _output) (`CameraComponent.FieldOfView` (`CameraActor.CameraComponent` _output))))

(fn `SetCameraPosition `
  (params (`New Transform` :type "Transform Structure") (`New Field Of View` :type "Float (double-precision)"))
  (`self.K2_SetActorTransform` `New Transform`)
  (`CameraComponent.SetFieldOfView` (`self.Camera`) `New Field Of View`))

(fn `UserConstructionScript`)
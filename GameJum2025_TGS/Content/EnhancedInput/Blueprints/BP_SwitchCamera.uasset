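; BP_SwitchCamera is a camera actor that becomes the player's view and moves between preset level cameras.
; On BeginPlay it takes over the view target and snaps to the transform and FOV of the first camera in the LevelCmaras array.
; SwitchCamera plays a timeline that interpolates transform and FOV from the current index's camera to the requested one, so a single camera blends between them rather than changing view targets.
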(event `self.ReceiveBeginPlay`
  (bind (_returnvalue _field_of_view) (`self.Get Camera Position` 0))
  (`PlayerController.SetViewTargetWithBlend` (`GameplayStatics.GetPlayerController` 0) self 0.0 "VTBlend_Linear" 0.0 false)
  (`self.Set Camera Position` _returnvalue _field_of_view))

(event `/Game/EnhancedInput/Blueprints/IF_CameraManager.SwitchCamera`
  (params (Index :type Integer))
  (bind (_returnvalue _field_of_view) (`self.Get Camera Position` Index))
  (bind (_returnvalue_2 _field_of_view_2) (`self.Get Camera Position` (`self.CurrentIndex`)))
  ;[1 1 1] New
  (set `self.NextTransform` _returnvalue)
  (set `self.NextFOV` _field_of_view)
  ;[1 1 1] Old
  (set `self.PreviousTransform` _returnvalue_2)
  (set `self.PreviousFOV` _field_of_view_2)
  (set `self.CurrentIndex` Index)
  (bind (_direction `_新規track_0`) (`Timeline|タイムライン` :!via `PlayFromStart`)
    (:`Update`
      (`self.Set Camera Position` (`KismetMathLibrary.TLerp` (`self.PreviousTransform`) (`self.NextTransform`) `_新規track_0`) (`KismetMathLibrary.Lerp` (`self.PreviousFOV`) (`self.NextFOV`) `_新規track_0`)))))

(fn `Get Camera Position`
  (params (Index :type Integer))
  (returns (ReturnValue :type "Transform Structure (by ref)") (`Field Of View` :type "Float (single-precision)"))
  (bind _output (`|GetArrayItem` (`self.LevelCmaras`) Index))
  (return (`self.GetTransform` _output) (`CameraComponent.FieldOfView` (`CameraActor.CameraComponent` _output))))

(fn `Set Camera Position`
  (params (NewTransform :type "Transform Structure (by ref)") (NewFieldOfView :type "Float (single-precision)"))
  (`self.K2_SetActorTransform` self NewTransform false false)
  (`CameraComponent.SetFieldOfView` (`self.Camera`) NewFieldOfView))

(fn `UserConstructionScript`)
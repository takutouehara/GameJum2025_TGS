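; BP_Shoulderbutton switches between two cameras with left and right input actions, as the name suggests for shoulder buttons.
; BeginPlay fills a Cameras array with Camera1 and Camera2.
; Each press steps CurrentCameraIndex down or up, clamps it, calls SetViewTargetWithBlend on the first player controller and calls Activate on Cameras.
; The clamp's upper bound is -1 and the view-target call receives no explicit target.
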(event `self.ReceiveBeginPlay`
  (`KismetArrayLibrary.Array_Add` (`self.Cameras`) (`self.Camera1`))
  (`KismetArrayLibrary.Array_Add` (`self.Cameras`) (`self.Camera2`)))

(event `InputAction|SwitchCameraLeft`
  (params (Key :type "Key Structure"))
  (:`Pressed`
    (bind _result (`/Engine/EditorBlueprintResources/StandardMacros.DecrementInt` (`self.CurrentCameraIndex`))
      (:`  `
        (set `self.CurrentCameraIndex` (`KismetMathLibrary.Clamp` _result 0 -1))
        (`self.SetViewTargetWithBlend` (`GameplayStatics.GetPlayerController` 0) null 0.0 "VTBlend_Linear" 0.0 false)
        (`ActorComponent.Activate` (`self.Cameras`) false)))))

(event `InputAction|SwitchCameraRight`
  (params (Key :type "Key Structure"))
  (:`Pressed`
    (bind _result (`/Engine/EditorBlueprintResources/StandardMacros.IncrementInt` (`self.CurrentCameraIndex`))
      (:`  `
        (set `self.CurrentCameraIndex` (`KismetMathLibrary.Clamp` _result 0 -1))
        (`self.SetViewTargetWithBlend` (`GameplayStatics.GetPlayerController` 0) null 0.0 "VTBlend_Linear" 0.0 false)
        (`ActorComponent.Activate` (`self.Cameras`) false)))))

(fn `UserConstructionScript`)
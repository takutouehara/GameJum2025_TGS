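; BP_RailCamera is a camera actor that rides a CameraRail spline while facing a TargetActor.
; Each Tick, while the target is valid, it places itself at DistanceAlongSpline, using local spline coordinates as its location, and turns via FindLookAtRotation.
; MoveCameraRight and MoveCameraLeft presses increment or decrement that distance, then overwrite it with a ClampFloat of constant zero, so the step is lost.
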(event `self.ReceiveTick`
  (params (DeltaSeconds :type "Float (single-precision)"))
  (`/Engine/EditorBlueprintResources/StandardMacros.IsValid` (`self.TargetActor`)
    (:`Is Valid`
      (`self.K2_SetActorLocation` (`SplineComponent.GetLocationAtDistanceAlongSpline` (`/Game/EnhancedInput/Blueprints/BP_CameraRail.Spline` (`self.CameraRail`)) (`self.DistanceAlongSpline`) "Local"))
      (`self.K2_SetActorRotation` (`KismetMathLibrary.FindLookAtRotation` (`self.K2_GetActorLocation`) (`self.K2_GetActorLocation` (`self.TargetActor`)))))))

(event `InputAction|MoveCameraRight`
  (params (Key :type "Key Structure"))
  (:`Pressed`
    (`/Engine/EditorBlueprintResources/StandardMacros.IncrementFloat` (`self.DistanceAlongSpline`)
      (:`  `
        (set `self.DistanceAlongSpline` (`KismetMathLibrary.FClamp` 0.0 0.0 10.0))))))

(event `InputAction|MoveCameraLeft`
  (params (Key :type "Key Structure"))
  (:`Pressed`
    (`/Engine/EditorBlueprintResources/StandardMacros.DecrementFloat` (`self.DistanceAlongSpline`)
      (:`  `
        (set `self.DistanceAlongSpline` (`KismetMathLibrary.FClamp` 0.0 0.0 -10.0))))))

(fn `UserConstructionScript`)
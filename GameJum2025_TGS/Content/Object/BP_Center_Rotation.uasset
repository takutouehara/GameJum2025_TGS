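; BP_Center_Rotation is an actor meant to turn itself a quarter turn about a chosen world axis.
; CenterX, CenterY and CenterZ events each set an axis flag.
; A disconnected sequence holds the stepping logic: delayed 10-degree world rotations, tallied by one shared counter that clears the flag after nine steps, with debug angle prints.
; Tick is empty and nothing triggers that sequence, so the actor never rotates as wired.
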(event `CenterX`
  (set `self.CheckerX` true))

(event `CenterY`
  (set `self.CheckerY` true))

(event `CenterZ`
  (set `self.CheckerZ` true))

(event `self.ReceiveTick`
  (params (DeltaSeconds :type "Float (single-precision)")))

(fn `UserConstructionScript`)
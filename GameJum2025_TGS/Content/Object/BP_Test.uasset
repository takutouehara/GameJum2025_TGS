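; BP_Test is a test actor holding unconnected logic to rotate a board piece around the BP_Center actor, labeled as X-axis rotation.
; The logic rotates the actor's offset from the center in fixed steps and applies a matching local rotation, with a counter capping the number of steps.
; No event drives this graph, so it never runs, and the construction script is empty.
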(fn `UserConstructionScript`)
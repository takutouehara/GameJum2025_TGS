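; Grid cursor for a turn-based piece-placing game that moves over the four vertical side faces of a cube.
; CurSor events teleport it one cell up or down within limits, or sideways via PositionLeft/PositionRight, which rotate it onto the adjacent face at edges using exact coordinate checks.
; ChangeColor swaps the plane's black/white material from the parity of MasterGameInstance's MasterCounter.
; Several older movement chains in the EventGraph are disconnected and never run.
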(event `CurSor Up`
  (bind _x (.x (`self.K2_GetActorLocation`)))
  (bind _y (.y (`self.K2_GetActorLocation`)))
  (if (< (.z (`self.K2_GetActorLocation`)) 150.0)
    (if (or (== _x -201.0) (== _y -201.0) (== _x 201.0) (== _y 201.0))
      (`self.K2_SetActorLocation` (`KismetMathLibrary.MakeVector` (.x (`self.K2_GetActorLocation`)) (.y (`self.K2_GetActorLocation`)) (+ (.z (`self.K2_GetActorLocation`)) 100.0)) false true))))

(event `self.ReceiveBeginPlay`)

(event `CurSor Down`
  (bind _x (.x (`self.K2_GetActorLocation`)))
  (bind _y (.y (`self.K2_GetActorLocation`)))
  (if (> (.z (`self.K2_GetActorLocation`)) -150.0)
    (if (or (== _x -201.0) (== _y -201.0) (== _x 201.0) (== _y 201.0))
      (`self.K2_SetActorLocation` (`KismetMathLibrary.MakeVector` (.x (`self.K2_GetActorLocation`)) (.y (`self.K2_GetActorLocation`)) (+ (.z (`self.K2_GetActorLocation`)) -100.0)) false true))))

(event `ChangeColor`
  ;[1 1 1] 設置するたびに駒の色を変える
  (bind _asmaster_game_instance (cast `/Game/MasterGameInstance` (`GameplayStatics.GetGameInstance`)))
  (if (== (mod (`/Game/MasterGameInstance.MasterCounter` _asmaster_game_instance) 2) 0)
    (`PrimitiveComponent.SetMaterial` (`self.Plane_cursor`) 0 "/Game/Material/MI_CursorKuro.MI_CursorKuro")
    (else
      (`PrimitiveComponent.SetMaterial` (`self.Plane_cursor`) 0 "/Game/Material/MI_CursorSiro.MI_CursorSiro"))))

(event `CurSor Left`
  ;[1 1 1] コメント
  (`self.Position Left`))

(event `CurSor Right`
  ;[1 1 1] コメント
  (`self.PositionRight`))

(fn `Position Left`
  (bind _x (.x (`self.K2_GetActorLocation`)))
  (bind _y (.y (`self.K2_GetActorLocation`)))
  (if (== _x -201.0)
    (`self.K2_SetActorLocation` (`KismetMathLibrary.MakeVector` (.x (`self.K2_GetActorLocation`)) (+ (.y (`self.K2_GetActorLocation`)) -100.0) (.z (`self.K2_GetActorLocation`))) false true)
    (if (== (.y (`self.K2_GetActorLocation`)) -250.0)
      (`self.K2_SetActorRotation` (`KismetMathLibrary.MakeRotator` 0.0 90.0 90.0))
      (`self.K2_SetActorLocation` (`KismetMathLibrary.MakeVector` (+ (.x (`self.K2_GetActorLocation`)) 51.0) (+ (.y (`self.K2_GetActorLocation`)) 49.0) (.z (`self.K2_GetActorLocation`))) false true))
    (elif (== _y -201.0)
      (`self.K2_SetActorLocation` (`KismetMathLibrary.MakeVector` (+ (.x (`self.K2_GetActorLocation`)) 100.0) (.y (`self.K2_GetActorLocation`)) (.z (`self.K2_GetActorLocation`))) false true)
      (if (== (.x (`self.K2_GetActorLocation`)) 250.0)
        (`self.K2_SetActorRotation` (`KismetMathLibrary.MakeRotator` 0.0 90.0 180.0))
        (`self.K2_SetActorLocation` (`KismetMathLibrary.MakeVector` (+ (.x (`self.K2_GetActorLocation`)) -49.0) (+ (.y (`self.K2_GetActorLocation`)) 51.0) (.z (`self.K2_GetActorLocation`))) false true))
      (elif (== _x 201.0)
        (`self.K2_SetActorLocation` (`KismetMathLibrary.MakeVector` (.x (`self.K2_GetActorLocation`)) (+ (.y (`self.K2_GetActorLocation`)) 100.0) (.z (`self.K2_GetActorLocation`))) false true)
        (if (== (.y (`self.K2_GetActorLocation`)) 250.0)
          (`self.K2_SetActorRotation` (`KismetMathLibrary.MakeRotator` 0.0 90.0 -90.0))
          (`self.K2_SetActorLocation` (`KismetMathLibrary.MakeVector` (+ (.x (`self.K2_GetActorLocation`)) -51.0) (+ (.y (`self.K2_GetActorLocation`)) -49.0) (.z (`self.K2_GetActorLocation`))) false true))
        (elif (== _y 201.0)
          (`self.K2_SetActorLocation` (`KismetMathLibrary.MakeVector` (+ (.x (`self.K2_GetActorLocation`)) -100.0) (.y (`self.K2_GetActorLocation`)) (.z (`self.K2_GetActorLocation`))) false true)
          (if (== (.x (`self.K2_GetActorLocation`)) -250.0)
            (`self.K2_SetActorRotation` (`KismetMathLibrary.MakeRotator` 0.0 90.0))
            (`self.K2_SetActorLocation` (`KismetMathLibrary.MakeVector` (+ (.x (`self.K2_GetActorLocation`)) 49.0) (+ (.y (`self.K2_GetActorLocation`)) -51.0) (.z (`self.K2_GetActorLocation`))) false true)))))))

(fn `PositionRight`
  (bind _x (.x (`self.K2_GetActorLocation`)))
  (bind _y (.y (`self.K2_GetActorLocation`)))
  (if (== _x -201.0)
    (`self.K2_SetActorLocation` (`KismetMathLibrary.MakeVector` (.x (`self.K2_GetActorLocation`)) (+ (.y (`self.K2_GetActorLocation`)) 100.0) (.z (`self.K2_GetActorLocation`))) false true)
    (if (== (.y (`self.K2_GetActorLocation`)) 250.0)
      (`self.K2_SetActorRotation` (`KismetMathLibrary.MakeRotator` 0.0 90.0 -90.0))
      (`self.K2_SetActorLocation` (`KismetMathLibrary.MakeVector` (+ (.x (`self.K2_GetActorLocation`)) 51.0) (+ (.y (`self.K2_GetActorLocation`)) -49.0) (.z (`self.K2_GetActorLocation`))) false true))
    (elif (== _y 201.0)
      (`self.K2_SetActorLocation` (`KismetMathLibrary.MakeVector` (+ (.x (`self.K2_GetActorLocation`)) 100.0) (.y (`self.K2_GetActorLocation`)) (.z (`self.K2_GetActorLocation`))) false true)
      (if (== (.x (`self.K2_GetActorLocation`)) 250.0)
        (`self.K2_SetActorRotation` (`KismetMathLibrary.MakeRotator` 0.0 90.0 180.0))
        (`self.K2_SetActorLocation` (`KismetMathLibrary.MakeVector` (+ (.x (`self.K2_GetActorLocation`)) -49.0) (+ (.y (`self.K2_GetActorLocation`)) -51.0) (.z (`self.K2_GetActorLocation`))) false true))
      (elif (== _x 201.0)
        (`self.K2_SetActorLocation` (`KismetMathLibrary.MakeVector` (.x (`self.K2_GetActorLocation`)) (+ (.y (`self.K2_GetActorLocation`)) -100.0) (.z (`self.K2_GetActorLocation`))) false true)
        (if (== (.y (`self.K2_GetActorLocation`)) -250.0)
          (`self.K2_SetActorRotation` (`KismetMathLibrary.MakeRotator` 0.0 90.0 90.0))
          (`self.K2_SetActorLocation` (`KismetMathLibrary.MakeVector` (+ (.x (`self.K2_GetActorLocation`)) -51.0) (+ (.y (`self.K2_GetActorLocation`)) 49.0) (.z (`self.K2_GetActorLocation`))) false true))
        (elif (== _y -201.0)
          (`self.K2_SetActorLocation` (`KismetMathLibrary.MakeVector` (+ (.x (`self.K2_GetActorLocation`)) -100.0) (.y (`self.K2_GetActorLocation`)) (.z (`self.K2_GetActorLocation`))) false true)
          (if (== (.x (`self.K2_GetActorLocation`)) -250.0)
            (`self.K2_SetActorRotation` (`KismetMathLibrary.MakeRotator` 0.0 90.0))
            (`self.K2_SetActorLocation` (`KismetMathLibrary.MakeVector` (+ (.x (`self.K2_GetActorLocation`)) 49.0) (+ (.y (`self.K2_GetActorLocation`)) 51.0) (.z (`self.K2_GetActorLocation`))) false true)))))))

(fn `UserConstructionScript`)
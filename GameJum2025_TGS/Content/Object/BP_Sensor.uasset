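; BP_Sensor is a stepping sensor actor with a Plane overlap that looks for BP_KomaObject actors.
; A Delay on Tick paces it to move 100 units along Y about every half second, at fixed X and Z, until a counter passes 10.
; The overlap handler only casts to BP_KomaObject and takes no action, and a gameplay tag comparison is left unconnected.
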(event `self.ReceiveTick`
  (params (DeltaSeconds :type "Float (single-precision)"))
  (`KismetSystemLibrary.Delay` 0.5)
  (if (<= (`self.Count`) 10)
    (`self.K2_SetActorLocation` (`KismetMathLibrary.MakeVector` 240.0 (+ (.y (`self.K2_GetActorLocation`)) 100.0) 600.0))
    (bind _result (`/Engine/EditorBlueprintResources/StandardMacros.IncrementInt` (`self.Count`))
      (:`  `
        (set `self.Count` _result)))))

(event `self.Plane.OnComponentBeginOverlap`
  (params (OverlappedComponent :type "PrimitiveComponent Object Reference") (OtherActor :type "Actor Object Reference") (OtherComp :type "PrimitiveComponent Object Reference") (OtherBodyIndex :type Integer) (bFromSweep :type Boolean) (SweepResult :type "HitResult Structure (by ref)"))
  (bind _asbp_koma_object (cast `/Game/Object/BP_KomaObject` OtherActor)))

(fn `UserConstructionScript`)
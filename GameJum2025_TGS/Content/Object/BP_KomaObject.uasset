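; Board-game piece actor that starts hidden and is revealed as a black or white piece where the cursor is.
; Box overlaps set OnCursor; Spawn then picks the material from MasterGameInstance's counter parity, unhides the piece, increments the counter and enables collision on 24 Core components.
; Reverse is an empty stub, edge-based timeline rotation and cursor-based SpawnActor placement are disconnected, and debug prints remain.
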(event `Reverse`
  ;[1 1 1] 駒の回転（右回転）
)

(event `self.ReceiveBeginPlay`
  ;[1 1 1] 開始時、すべての駒を不可視化する
  (`self.SetActorHiddenInGame` true))

(event `self.Box.OnComponentBeginOverlap`
  (params (OverlappedComponent :type "PrimitiveComponent Object Reference") (OtherActor :type "Actor Object Reference") (OtherComp :type "PrimitiveComponent Object Reference") (OtherBodyIndex :type Integer) (bFromSweep :type Boolean) (SweepResult :type "HitResult Structure (by ref)"))
  ;[1 1 1] 不可視化されている駒とカーソルが接触した
  (set `self.on Cursor` true))

(event `self.Box.OnComponentEndOverlap`
  (params (OverlappedComponent :type "PrimitiveComponent Object Reference") (OtherActor :type "Actor Object Reference") (OtherComp :type "PrimitiveComponent Object Reference") (OtherBodyIndex :type Integer))
  ;[1 1 1] 不可視化されている駒とカーソルが離れた
  (set `self.on Cursor` false))

(event `Spawn`
  (if (`self.on Cursor`)
    (if (`self.bHidden`)
      (bind _asmaster_game_instance (cast `/Game/MasterGameInstance` (`GameplayStatics.GetGameInstance`)))
      (if (== (mod (`/Game/MasterGameInstance.MasterCounter` _asmaster_game_instance) 2) 0)
        (`PrimitiveComponent.SetMaterial` (`self.StaticMesh`) 0 "/Game/Material/MI_Kuro.MI_Kuro")
        (else
          (`PrimitiveComponent.SetMaterial` (`self.StaticMesh`) 0 "/Game/Material/MI_Siro.MI_Siro")))
      (`self.SetActorHiddenInGame` false)
      (bind _asmaster_game_instance_2 (cast `/Game/MasterGameInstance` (`GameplayStatics.GetGameInstance`)))
      (bind _result (`/Engine/EditorBlueprintResources/StandardMacros.IncrementInt` (`/Game/MasterGameInstance.MasterCounter` _asmaster_game_instance_2))
        (:`  `
          (set `/Game/MasterGameInstance.MasterCounter` _result _asmaster_game_instance_2)
          (`PrimitiveComponent.SetCollisionEnabled` (`self.core_1`) "QueryAndPhysics")
          (`PrimitiveComponent.SetCollisionEnabled` (`self.core_2`) "QueryAndPhysics")
          (`PrimitiveComponent.SetCollisionEnabled` (`self.core_3`) "QueryAndPhysics")
          (`PrimitiveComponent.SetCollisionEnabled` (`self.core_4`) "QueryAndPhysics")
          (`PrimitiveComponent.SetCollisionEnabled` (`self.core_5`) "QueryAndPhysics")
          (`PrimitiveComponent.SetCollisionEnabled` (`self.core_6`) "QueryAndPhysics")
          (`PrimitiveComponent.SetCollisionEnabled` (`self.core_7`) "QueryAndPhysics")
          (`PrimitiveComponent.SetCollisionEnabled` (`self.core_8`) "QueryAndPhysics")
          (`PrimitiveComponent.SetCollisionEnabled` (`self.core_9`) "QueryAndPhysics")
          (`PrimitiveComponent.SetCollisionEnabled` (`self.core_10`) "QueryAndPhysics")
          (`PrimitiveComponent.SetCollisionEnabled` (`self.core_11`) "QueryAndPhysics")
          (`PrimitiveComponent.SetCollisionEnabled` (`self.core_12`) "QueryAndPhysics")
          (`PrimitiveComponent.SetCollisionEnabled` (`self.core_13`) "QueryAndPhysics")
          (`PrimitiveComponent.SetCollisionEnabled` (`self.core_14`) "QueryAndPhysics")
          (`PrimitiveComponent.SetCollisionEnabled` (`self.core_15`) "QueryAndPhysics")
          (`PrimitiveComponent.SetCollisionEnabled` (`self.core_16`) "QueryAndPhysics")
          (`PrimitiveComponent.SetCollisionEnabled` (`self.core_17`) "QueryAndPhysics")
          (`PrimitiveComponent.SetCollisionEnabled` (`self.core_18`) "QueryAndPhysics")
          (`PrimitiveComponent.SetCollisionEnabled` (`self.core_19`) "QueryAndPhysics")
          (`PrimitiveComponent.SetCollisionEnabled` (`self.core_20`) "QueryAndPhysics")
          (`PrimitiveComponent.SetCollisionEnabled` (`self.core_21`) "QueryAndPhysics")
          (`PrimitiveComponent.SetCollisionEnabled` (`self.core_22`) "QueryAndPhysics")
          (`PrimitiveComponent.SetCollisionEnabled` (`self.core_23`) "QueryAndPhysics")
          (`PrimitiveComponent.SetCollisionEnabled` (`self.core_24`) "QueryAndPhysics"))))))

(event `Debugbug`
  (bind _asmaster_game_instance (cast `/Game/MasterGameInstance` (`GameplayStatics.GetGameInstance`)))
  (`KismetSystemLibrary.PrintString` (`KismetStringLibrary.Conv_IntToString` (`/Game/MasterGameInstance.MasterCounter` _asmaster_game_instance))))

(event `self.core_13.OnComponentBeginOverlap`
  (params (OverlappedComponent :type "PrimitiveComponent Object Reference") (OtherActor :type "Actor Object Reference") (OtherComp :type "PrimitiveComponent Object Reference") (OtherBodyIndex :type Integer) (bFromSweep :type Boolean) (SweepResult :type "HitResult Structure (by ref)"))
  (`KismetSystemLibrary.PrintString` "Hello"))

(fn `UserConstructionScript`)
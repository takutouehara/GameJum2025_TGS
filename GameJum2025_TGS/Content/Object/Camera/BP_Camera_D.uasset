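; BP_Camera_D is a camera actor that sets its orientation to match the currently active side, apparently for a downward view.
; Its DownCamera event casts the game instance to MasterGameInstance and checks the front, left, back and right side flags in that priority order.
; The first true flag snaps the actor to a matching quarter-turn rotation about a single axis, and no set flag leaves it unchanged.
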(event `DownCamera`
  (bind _asmaster_game_instance (cast `/Game/MasterGameInstance` (`GameplayStatics.GetGameInstance`)))
  (if (`/Game/MasterGameInstance.FrontSide` _asmaster_game_instance)
    (`self.K2_SetActorRotation` (struct))
    (elif (`/Game/MasterGameInstance.LeftSide` _asmaster_game_instance)
      (`self.K2_SetActorRotation` (struct :`Yaw` 90.0))
      (elif (`/Game/MasterGameInstance.BackSide` _asmaster_game_instance)
        (`self.K2_SetActorRotation` (struct :`Yaw` 180.0))
        (elif (`/Game/MasterGameInstance.RightSide` _asmaster_game_instance)
          (`self.K2_SetActorRotation` (struct :`Yaw` -90.0)))))))

(fn `UserConstructionScript`)
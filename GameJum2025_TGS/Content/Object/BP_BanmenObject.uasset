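; Board piece that makes animated quarter turns around BP_Center, in the manner of a Rubik's Cube slice.
; Twelve Rotation events each match one X, Y or Z layer by actor location and set a flag for that axis.
; Tick runs collapsed per-axis graphs that orbit and rotate the piece in nine delayed 10-degree steps.
; On completion they reset the flag and counter, update both cursors' colors and clear MoveNow on MasterGameInstance.
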(event `Rotation 1`
  ;[1 1 1] コメント
  (if (`KismetMathLibrary.NearlyEqual_FloatFloat` (.y (`self.K2_GetActorLocation`)) -150.0 0.001)
    (set `self.Checker Y-150` true)))

(event `Rotation 2`
  ;[1 1 1] コメント
  (if (`KismetMathLibrary.NearlyEqual_FloatFloat` (.y (`self.K2_GetActorLocation`)) -50.0 0.001)
    (set `self.Checker Y-50` true)))

(event `Rotation 3`
  ;[1 1 1] コメント
  (if (`KismetMathLibrary.NearlyEqual_FloatFloat` (.y (`self.K2_GetActorLocation`)) 50.0 0.001)
    (set `self.Checker Y50` true)))

(event `Rotation 4`
  ;[1 1 1] コメント
  (if (`KismetMathLibrary.NearlyEqual_FloatFloat` (.y (`self.K2_GetActorLocation`)) 150.0 0.001)
    (set `self.Checker Y150` true)))

(event `self.ReceiveTick`
  (params (DeltaSeconds :type "Float (single-precision)"))
  ;[1 1 1] 回転処理
  (`|ExecutionSequence`
    (:`then_0`
      (`|ExecutionSequence`
        (:`then_0`
          (if (`self.Checker Y-150`)
            (if (< (`self.RowlingCounter`) 9)
              (bind _returnvalue (`GameplayStatics.GetActorOfClass` "/Game/Object/BP_Center.BP_Center_C"))
              (`KismetSystemLibrary.Delay` 0.1)
              (bind _result (`/Engine/EditorBlueprintResources/StandardMacros.IncrementInt` (`self.RowlingCounter`))
                (:`  `
                  (set `self.RowlingCounter` _result)
                  (bind _returnvalue_2 (`self.K2_GetActorLocation` _returnvalue))
                  (`self.K2_SetActorLocation` (+ (`KismetMathLibrary.GreaterGreater_VectorRotator` (- (`self.K2_GetActorLocation`) _returnvalue_2) (struct :`Pitch` 10.0)) _returnvalue_2) false true)
                  (`self.K2_AddActorWorldRotation` (struct :`Pitch` 10.0))))
              (else
                (set `self.Checker Y-150` false)
                (set `self.RowlingCounter` 0)
                (`self.ChangeColor`)
                (bind _asmaster_game_instance (cast `/Game/MasterGameInstance` (`GameplayStatics.GetGameInstance`) :!label _label))
                (set `/Game/MasterGameInstance.MoveNow` false _asmaster_game_instance)))))
        (:`then_1`
          (if (`self.Checker Y-50`)
            (if (< (`self.RowlingCounter`) 9)
              (bind _returnvalue_3 (`GameplayStatics.GetActorOfClass` "/Game/Object/BP_Center.BP_Center_C"))
              (`KismetSystemLibrary.Delay` 0.1)
              (bind _result_2 (`/Engine/EditorBlueprintResources/StandardMacros.IncrementInt` (`self.RowlingCounter`))
                (:`  `
                  (set `self.RowlingCounter` _result_2)
                  (bind _returnvalue_4 (`self.K2_GetActorLocation` _returnvalue_3))
                  (`self.K2_SetActorLocation` (+ (`KismetMathLibrary.GreaterGreater_VectorRotator` (- (`self.K2_GetActorLocation`) _returnvalue_4) (struct :`Pitch` 10.0)) _returnvalue_4) false true)
                  (`self.K2_AddActorWorldRotation` (struct :`Pitch` 10.0))))
              (else
                (set `self.Checker Y-50` false)
                (set `self.RowlingCounter` 0)
                (`self.ChangeColor`)
                (goto _label)))))
        (:`then_2`
          (if (`self.Checker Y50`)
            (if (< (`self.RowlingCounter`) 9)
              (bind _returnvalue_5 (`GameplayStatics.GetActorOfClass` "/Game/Object/BP_Center.BP_Center_C"))
              (`KismetSystemLibrary.Delay` 0.1)
              (bind _result_3 (`/Engine/EditorBlueprintResources/StandardMacros.IncrementInt` (`self.RowlingCounter`))
                (:`  `
                  (set `self.RowlingCounter` _result_3)
                  (bind _returnvalue_6 (`self.K2_GetActorLocation` _returnvalue_5))
                  (`self.K2_SetActorLocation` (+ (`KismetMathLibrary.GreaterGreater_VectorRotator` (- (`self.K2_GetActorLocation`) _returnvalue_6) (struct :`Pitch` 10.0)) _returnvalue_6) false true)
                  (`self.K2_AddActorWorldRotation` (struct :`Pitch` 10.0))))
              (else
                (set `self.Checker Y50` false)
                (set `self.RowlingCounter` 0)
                (`self.ChangeColor`)
                (goto _label)))))
        (:`then_3`
          (if (`self.Checker Y150`)
            (if (< (`self.RowlingCounter`) 9)
              (bind _returnvalue_7 (`GameplayStatics.GetActorOfClass` "/Game/Object/BP_Center.BP_Center_C"))
              (`KismetSystemLibrary.Delay` 0.1)
              (bind _result_4 (`/Engine/EditorBlueprintResources/StandardMacros.IncrementInt` (`self.RowlingCounter`))
                (:`  `
                  (set `self.RowlingCounter` _result_4)
                  (bind _returnvalue_8 (`self.K2_GetActorLocation` _returnvalue_7))
                  (`self.K2_SetActorLocation` (+ (`KismetMathLibrary.GreaterGreater_VectorRotator` (- (`self.K2_GetActorLocation`) _returnvalue_8) (struct :`Pitch` 10.0)) _returnvalue_8) false true)
                  (`self.K2_AddActorWorldRotation` (struct :`Pitch` 10.0))))
              (else
                (set `self.Checker Y150` false)
                (set `self.RowlingCounter` 0)
                (`self.ChangeColor`)
                (goto _label)))))))
    (:`then_1`
      (`|ExecutionSequence`
        (:`then_0`
          (if (`self.Checker X-150`)
            (if (< (`self.RowlingCounter`) 9)
              (bind _returnvalue_9 (`GameplayStatics.GetActorOfClass` "/Game/Object/BP_Center.BP_Center_C"))
              (`KismetSystemLibrary.Delay` 0.1)
              (bind _result_5 (`/Engine/EditorBlueprintResources/StandardMacros.IncrementInt` (`self.RowlingCounter`))
                (:`  `
                  (set `self.RowlingCounter` _result_5)
                  (bind _returnvalue_10 (`self.K2_GetActorLocation` _returnvalue_9))
                  (`self.K2_SetActorLocation` (+ (`KismetMathLibrary.GreaterGreater_VectorRotator` (- (`self.K2_GetActorLocation`) _returnvalue_10) (struct :`Roll` 10.0)) _returnvalue_10) false true)
                  (`self.K2_AddActorWorldRotation` (struct :`Roll` 10.0))))
              (else
                (set `self.Checker X-150` false)
                (set `self.RowlingCounter` 0)
                (`self.ChangeColor`)
                (goto _label)))))
        (:`then_1`
          (if (`self.Checker X-50`)
            (if (< (`self.RowlingCounter`) 9)
              (bind _returnvalue_11 (`GameplayStatics.GetActorOfClass` "/Game/Object/BP_Center.BP_Center_C"))
              (`KismetSystemLibrary.Delay` 0.1)
              (bind _result_6 (`/Engine/EditorBlueprintResources/StandardMacros.IncrementInt` (`self.RowlingCounter`))
                (:`  `
                  (set `self.RowlingCounter` _result_6)
                  (bind _returnvalue_12 (`self.K2_GetActorLocation` _returnvalue_11))
                  (`self.K2_SetActorLocation` (+ (`KismetMathLibrary.GreaterGreater_VectorRotator` (- (`self.K2_GetActorLocation`) _returnvalue_12) (struct :`Roll` 10.0)) _returnvalue_12) false true)
                  (`self.K2_AddActorWorldRotation` (struct :`Roll` 10.0))))
              (else
                (set `self.Checker X-50` false)
                (set `self.RowlingCounter` 0)
                (`self.ChangeColor`)
                (goto _label)))))
        (:`then_2`
          (if (`self.Checker X50`)
            (if (< (`self.RowlingCounter`) 9)
              (bind _returnvalue_13 (`GameplayStatics.GetActorOfClass` "/Game/Object/BP_Center.BP_Center_C"))
              (`KismetSystemLibrary.Delay` 0.1)
              (bind _result_7 (`/Engine/EditorBlueprintResources/StandardMacros.IncrementInt` (`self.RowlingCounter`))
                (:`  `
                  (set `self.RowlingCounter` _result_7)
                  (bind _returnvalue_14 (`self.K2_GetActorLocation` _returnvalue_13))
                  (`self.K2_SetActorLocation` (+ (`KismetMathLibrary.GreaterGreater_VectorRotator` (- (`self.K2_GetActorLocation`) _returnvalue_14) (struct :`Roll` 10.0)) _returnvalue_14) false true)
                  (`self.K2_AddActorWorldRotation` (struct :`Roll` 10.0))))
              (else
                (set `self.Checker X50` false)
                (set `self.RowlingCounter` 0)
                (`self.ChangeColor`)
                (goto _label)))))
        (:`then_3`
          (if (`self.Checker X150`)
            (if (< (`self.RowlingCounter`) 9)
              (bind _returnvalue_15 (`GameplayStatics.GetActorOfClass` "/Game/Object/BP_Center.BP_Center_C"))
              (`KismetSystemLibrary.Delay` 0.1)
              (bind _result_8 (`/Engine/EditorBlueprintResources/StandardMacros.IncrementInt` (`self.RowlingCounter`))
                (:`  `
                  (set `self.RowlingCounter` _result_8)
                  (bind _returnvalue_16 (`self.K2_GetActorLocation` _returnvalue_15))
                  (`self.K2_SetActorLocation` (+ (`KismetMathLibrary.GreaterGreater_VectorRotator` (- (`self.K2_GetActorLocation`) _returnvalue_16) (struct :`Roll` 10.0)) _returnvalue_16) false true)
                  (`self.K2_AddActorWorldRotation` (struct :`Roll` 10.0))))
              (else
                (set `self.Checker X150` false)
                (set `self.RowlingCounter` 0)
                (`self.ChangeColor`)
                (goto _label)))))))
    (:`then_2`
      (`|ExecutionSequence`
        (:`then_0`
          (if (`self.Checker Z-150`)
            (if (< (`self.RowlingCounter`) 9)
              (bind _returnvalue_17 (`GameplayStatics.GetActorOfClass` "/Game/Object/BP_Center.BP_Center_C"))
              (`KismetSystemLibrary.Delay` 0.1)
              (bind _result_9 (`/Engine/EditorBlueprintResources/StandardMacros.IncrementInt` (`self.RowlingCounter`))
                (:`  `
                  (set `self.RowlingCounter` _result_9)
                  (bind _returnvalue_18 (`self.K2_GetActorLocation` _returnvalue_17))
                  (`self.K2_SetActorLocation` (+ (`KismetMathLibrary.GreaterGreater_VectorRotator` (- (`self.K2_GetActorLocation`) _returnvalue_18) (struct :`Yaw` 10.0)) _returnvalue_18) false true)
                  (`self.K2_AddActorWorldRotation` (struct :`Yaw` 10.0))))
              (else
                (set `self.Checker Z-150` false)
                (set `self.RowlingCounter` 0)
                (`self.ChangeColor`)
                (goto _label)))))
        (:`then_1`
          (if (`self.Checker Z-50`)
            (if (< (`self.RowlingCounter`) 9)
              (bind _returnvalue_19 (`GameplayStatics.GetActorOfClass` "/Game/Object/BP_Center.BP_Center_C"))
              (`KismetSystemLibrary.Delay` 0.1)
              (bind _result_10 (`/Engine/EditorBlueprintResources/StandardMacros.IncrementInt` (`self.RowlingCounter`))
                (:`  `
                  (set `self.RowlingCounter` _result_10)
                  (bind _returnvalue_20 (`self.K2_GetActorLocation` _returnvalue_19))
                  (`self.K2_SetActorLocation` (+ (`KismetMathLibrary.GreaterGreater_VectorRotator` (- (`self.K2_GetActorLocation`) _returnvalue_20) (struct :`Yaw` 10.0)) _returnvalue_20) false true)
                  (`self.K2_AddActorWorldRotation` (struct :`Yaw` 10.0))))
              (else
                (set `self.Checker Z-50` false)
                (set `self.RowlingCounter` 0)
                (`self.ChangeColor`)
                (goto _label)))))
        (:`then_2`
          (if (`self.Checker Z50`)
            (if (< (`self.RowlingCounter`) 9)
              (bind _returnvalue_21 (`GameplayStatics.GetActorOfClass` "/Game/Object/BP_Center.BP_Center_C"))
              (`KismetSystemLibrary.Delay` 0.1)
              (bind _result_11 (`/Engine/EditorBlueprintResources/StandardMacros.IncrementInt` (`self.RowlingCounter`))
                (:`  `
                  (set `self.RowlingCounter` _result_11)
                  (bind _returnvalue_22 (`self.K2_GetActorLocation` _returnvalue_21))
                  (`self.K2_SetActorLocation` (+ (`KismetMathLibrary.GreaterGreater_VectorRotator` (- (`self.K2_GetActorLocation`) _returnvalue_22) (struct :`Yaw` 10.0)) _returnvalue_22) false true)
                  (`self.K2_AddActorWorldRotation` (struct :`Yaw` 10.0))))
              (else
                (set `self.Checker Z50` false)
                (set `self.RowlingCounter` 0)
                (`self.ChangeColor`)
                (goto _label)))))
        (:`then_3`
          (if (`self.Checker Z150`)
            (if (< (`self.RowlingCounter`) 9)
              (bind _returnvalue_23 (`GameplayStatics.GetActorOfClass` "/Game/Object/BP_Center.BP_Center_C"))
              (`KismetSystemLibrary.Delay` 0.1)
              (bind _result_12 (`/Engine/EditorBlueprintResources/StandardMacros.IncrementInt` (`self.RowlingCounter`))
                (:`  `
                  (set `self.RowlingCounter` _result_12)
                  (bind _returnvalue_24 (`self.K2_GetActorLocation` _returnvalue_23))
                  (`self.K2_SetActorLocation` (+ (`KismetMathLibrary.GreaterGreater_VectorRotator` (- (`self.K2_GetActorLocation`) _returnvalue_24) (struct :`Yaw` 10.0)) _returnvalue_24) false true)
                  (`self.K2_AddActorWorldRotation` (struct :`Yaw` 10.0))))
              (else
                (set `self.Checker Z150` false)
                (set `self.RowlingCounter` 0)
                (`self.ChangeColor`)
                (goto _label)))))))))

(event `Rotation 5`
  ;[1 1 1] コメント
  (if (`KismetMathLibrary.NearlyEqual_FloatFloat` (.x (`self.K2_GetActorLocation`)) -150.0 0.001)
    (set `self.Checker X-150` true)))

(event `Rotation 6`
  ;[1 1 1] コメント
  (if (`KismetMathLibrary.NearlyEqual_FloatFloat` (.x (`self.K2_GetActorLocation`)) -50.0 0.001)
    (set `self.Checker X-50` true)))

(event `Rotation 7`
  ;[1 1 1] コメント
  (if (`KismetMathLibrary.NearlyEqual_FloatFloat` (.x (`self.K2_GetActorLocation`)) 50.0 0.001)
    (set `self.Checker X50` true)))

(event `Rotation 8`
  ;[1 1 1] コメント
  (if (`KismetMathLibrary.NearlyEqual_FloatFloat` (.x (`self.K2_GetActorLocation`)) 150.0 0.001)
    (set `self.Checker X150` true)))

(event `Rotation 9`
  ;[1 1 1] コメント
  (if (`KismetMathLibrary.NearlyEqual_FloatFloat` (.z (`self.K2_GetActorLocation`)) -150.0 0.001)
    (set `self.Checker Z-150` true)))

(event `Rotation 10`
  ;[1 1 1] コメント
  (if (`KismetMathLibrary.NearlyEqual_FloatFloat` (.z (`self.K2_GetActorLocation`)) -50.0 0.001)
    (set `self.Checker Z-50` true)))

(event `Rotation 11`
  ;[1 1 1] コメント
  (if (`KismetMathLibrary.NearlyEqual_FloatFloat` (.z (`self.K2_GetActorLocation`)) 50.0 0.001)
    (set `self.Checker Z50` true)))

(event `Rotation 12`
  ;[1 1 1] コメント
  (if (`KismetMathLibrary.NearlyEqual_FloatFloat` (.z (`self.K2_GetActorLocation`)) 150.0 0.001)
    (set `self.Checker Z150` true)))

(fn `ChangeColor`
  (bind _returnvalue (`GameplayStatics.GetActorOfClass` "/Game/Object/BP_Cursor.BP_Cursor_C"))
  (`/Game/Object/BP_Cursor.ChangeColor` _returnvalue)
  (bind _returnvalue_2 (`GameplayStatics.GetActorOfClass` "/Game/Object/BP_CursorLarge.BP_CursorLarge_C"))
  (`/Game/Object/BP_CursorLarge.ChangeColorLarge` _returnvalue_2))

(fn `UserConstructionScript`)
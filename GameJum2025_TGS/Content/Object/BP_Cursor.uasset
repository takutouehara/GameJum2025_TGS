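; Cursor actor that steps across the six faces of a cube grid, marking where the next piece is placed.
; Tick shows or hides it from the game instance's CursorMode, and ChangeColor swaps black and white materials by MasterChecker parity.
; Four direction events teleport it one cell, detecting the current face by exact coordinate comparisons and wrapping over edges by re-offsetting and rotating onto the adjacent face.
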(event `self.ReceiveTick`
  (params (DeltaSeconds :type "Float (single-precision)"))
  ;[1 1 1] コメント
  (bind _asmaster_game_instance (cast `/Game/MasterGameInstance` (`GameplayStatics.GetGameInstance`)))
  (if (`/Game/MasterGameInstance.CursorMode` _asmaster_game_instance)
    (`self.SetActorHiddenInGame` false)
    (else
      (`self.SetActorHiddenInGame` true))))

(event `self.ReceiveBeginPlay`
  ;[1 1 1] カーソルの初期配置
  (`KismetSystemLibrary.Delay` 0.1)
  (`self.K2_SetActorLocation` (-201.0 150.0 150.0) false true)
  (`self.K2_SetActorRotation` (`KismetMathLibrary.MakeRotator` 0.0 90.0)))

(event `ChangeColor`
  ;[1 1 1] 設置するたびにカーソルの色を変える
  (bind _asmaster_game_instance (cast `/Game/MasterGameInstance` (`GameplayStatics.GetGameInstance`)))
  (if (== (mod (`/Game/MasterGameInstance.MasterChecker` _asmaster_game_instance) 2) 0)
    (`PrimitiveComponent.SetMaterial` (`self.Plane_cursor`) 0 "/Game/Material/MI_CursorKuro.MI_CursorKuro")
    (else
      (`PrimitiveComponent.SetMaterial` (`self.Plane_cursor`) 0 "/Game/Material/MI_CursorSiro.MI_CursorSiro"))))

(event `CurSor Up`
  ;[1 1 1] カーソル操作
  (`self.PositionUp`))

(event `CurSor Left`
  ;[1 1 1] カーソル操作
  (`self.Position Left`))

(event `CurSor Down`
  ;[1 1 1] カーソル操作
  (`self.PositionDown`))

(event `CurSor Right`
  ;[1 1 1] カーソル操作
  (`self.PositionRight`))

(fn `Position Left`
  (bind _x (.x (`self.K2_GetActorLocation`)))
  (bind _y (.y (`self.K2_GetActorLocation`)))
  (if (== _x -201.0)
    (`self.K2_SetActorLocation` (`KismetMathLibrary.MakeVector` (.x (`self.K2_GetActorLocation`)) (+ (.y (`self.K2_GetActorLocation`)) -100.0) (.z (`self.K2_GetActorLocation`))) false true)
    (if (== (.y (`self.K2_GetActorLocation`)) -250.0)
      (`self.K2_SetActorRotation` (`KismetMathLibrary.MakeRotator` 0.0 90.0 90.0))
      (`self.K2_SetActorLocation` (`KismetMathLibrary.MakeVector` (+ (.x (`self.K2_GetActorLocation`)) 51.0) (+ (.y (`self.K2_GetActorLocation`)) 49.0) (.z (`self.K2_GetActorLocation`))) false true))
    (elif (== _y -201.0)
      (`self.K2_SetActorLocation` (`KismetMathLibrary.MakeVector` (+ (.x (`self.K2_GetActorLocation`)) 100.0) (.y (`self.K2_GetActorLocation`)) (.z (`self.K2_GetActorLocation`))) false true)
      (if (== (.x (`self.K2_GetActorLocation`)) 250.0)
        (`self.K2_SetActorRotation` (`KismetMathLibrary.MakeRotator` 0.0 90.0 180.0))
        (`self.K2_SetActorLocation` (`KismetMathLibrary.MakeVector` (+ (.x (`self.K2_GetActorLocation`)) -49.0) (+ (.y (`self.K2_GetActorLocation`)) 51.0) (.z (`self.K2_GetActorLocation`))) false true))
      (elif (== _x 201.0)
        (`self.K2_SetActorLocation` (`KismetMathLibrary.MakeVector` (.x (`self.K2_GetActorLocation`)) (+ (.y (`self.K2_GetActorLocation`)) 100.0) (.z (`self.K2_GetActorLocation`))) false true)
        (if (== (.y (`self.K2_GetActorLocation`)) 250.0)
          (`self.K2_SetActorRotation` (`KismetMathLibrary.MakeRotator` 0.0 90.0 -90.0))
          (`self.K2_SetActorLocation` (`KismetMathLibrary.MakeVector` (+ (.x (`self.K2_GetActorLocation`)) -51.0) (+ (.y (`self.K2_GetActorLocation`)) -49.0) (.z (`self.K2_GetActorLocation`))) false true))
        (elif (== _y 201.0)
          (`self.K2_SetActorLocation` (`KismetMathLibrary.MakeVector` (+ (.x (`self.K2_GetActorLocation`)) -100.0) (.y (`self.K2_GetActorLocation`)) (.z (`self.K2_GetActorLocation`))) false true)
          (if (== (.x (`self.K2_GetActorLocation`)) -250.0)
            (`self.K2_SetActorRotation` (`KismetMathLibrary.MakeRotator` 0.0 90.0))
            (`self.K2_SetActorLocation` (`KismetMathLibrary.MakeVector` (+ (.x (`self.K2_GetActorLocation`)) 49.0) (+ (.y (`self.K2_GetActorLocation`)) -51.0) (.z (`self.K2_GetActorLocation`))) false true))
          (elif (== (.z (`self.K2_GetActorLocation`)) 201.0)
            (`self.K2_SetActorLocation` (`KismetMathLibrary.MakeVector` (.x (`self.K2_GetActorLocation`)) (+ (.y (`self.K2_GetActorLocation`)) -100.0) (.z (`self.K2_GetActorLocation`))) false true)
            (if (== (.y (`self.K2_GetActorLocation`)) -250.0)
              (`self.K2_SetActorRotation` (`KismetMathLibrary.MakeRotator` -90.0))
              (`self.K2_SetActorLocation` (`KismetMathLibrary.MakeVector` (.x (`self.K2_GetActorLocation`)) (+ (.y (`self.K2_GetActorLocation`)) 49.0) (+ (.z (`self.K2_GetActorLocation`)) -51.0)) false true))
            (elif (== (.z (`self.K2_GetActorLocation`)) -201.0)
              (`self.K2_SetActorLocation` (`KismetMathLibrary.MakeVector` (.x (`self.K2_GetActorLocation`)) (+ (.y (`self.K2_GetActorLocation`)) -100.0) (.z (`self.K2_GetActorLocation`))) false true)
              (if (== (.y (`self.K2_GetActorLocation`)) -250.0)
                (`self.K2_SetActorRotation` (`KismetMathLibrary.MakeRotator` -90.0))
                (`self.K2_SetActorLocation` (`KismetMathLibrary.MakeVector` (.x (`self.K2_GetActorLocation`)) (+ (.y (`self.K2_GetActorLocation`)) 49.0) (+ (.z (`self.K2_GetActorLocation`)) 51.0)) false true)))))))))

(fn `PositionDown`
  (bind _x (.x (`self.K2_GetActorLocation`)))
  (bind _y (.y (`self.K2_GetActorLocation`)))
  (bind _x_2 (.x (`self.K2_GetActorLocation`)))
  (bind _y_2 (.y (`self.K2_GetActorLocation`)))
  (if (or (== _x_2 -201.0) (== _y_2 -201.0) (== _x_2 201.0) (== _y_2 201.0))
    (`self.K2_SetActorLocation` (`KismetMathLibrary.MakeVector` (.x (`self.K2_GetActorLocation`)) (.y (`self.K2_GetActorLocation`)) (+ (.z (`self.K2_GetActorLocation`)) -100.0)) false true)
    (if (== (.z (`self.K2_GetActorLocation`)) -250.0)
      (if (== _x -201.0)
        (`self.K2_SetActorRotation` (`KismetMathLibrary.MakeRotator` 180.0))
        (`self.K2_SetActorLocation` (`KismetMathLibrary.MakeVector` (+ (.x (`self.K2_GetActorLocation`)) 51.0) (.y (`self.K2_GetActorLocation`)) (+ (.z (`self.K2_GetActorLocation`)) 49.0)) false true)
        (elif (== _y -201.0)
          (`self.K2_SetActorRotation` (`KismetMathLibrary.MakeRotator` 180.0))
          (`self.K2_SetActorLocation` (`KismetMathLibrary.MakeVector` (.x (`self.K2_GetActorLocation`)) (+ (.y (`self.K2_GetActorLocation`)) 51.0) (+ (.z (`self.K2_GetActorLocation`)) 49.0)) false true)
          (elif (== _x 201.0)
            (`self.K2_SetActorRotation` (`KismetMathLibrary.MakeRotator` 180.0))
            (`self.K2_SetActorLocation` (`KismetMathLibrary.MakeVector` (+ (.x (`self.K2_GetActorLocation`)) -51.0) (.y (`self.K2_GetActorLocation`)) (+ (.z (`self.K2_GetActorLocation`)) 49.0)) false true)
            (elif (== _y 201.0)
              (`self.K2_SetActorRotation` (`KismetMathLibrary.MakeRotator` 180.0))
              (`self.K2_SetActorLocation` (`KismetMathLibrary.MakeVector` (.x (`self.K2_GetActorLocation`)) (+ (.y (`self.K2_GetActorLocation`)) -51.0) (+ (.z (`self.K2_GetActorLocation`)) 49.0)) false true))))))
    (elif (== (.z (`self.K2_GetActorLocation`)) -201.0)
      (`self.K2_SetActorLocation` (`KismetMathLibrary.MakeVector` (+ (.x (`self.K2_GetActorLocation`)) 100.0) (.y (`self.K2_GetActorLocation`)) (.z (`self.K2_GetActorLocation`))) false true)
      (if (== (.x (`self.K2_GetActorLocation`)) 250.0)
        (`self.K2_SetActorRotation` (`KismetMathLibrary.MakeRotator` 0.0 90.0 180.0))
        (`self.K2_SetActorLocation` (`KismetMathLibrary.MakeVector` (+ (.x (`self.K2_GetActorLocation`)) -49.0) (.y (`self.K2_GetActorLocation`)) (+ (.z (`self.K2_GetActorLocation`)) 51.0)) false true))
      (elif (== (.z (`self.K2_GetActorLocation`)) 201.0)
        (`self.K2_SetActorLocation` (`KismetMathLibrary.MakeVector` (+ (.x (`self.K2_GetActorLocation`)) -100.0) (.y (`self.K2_GetActorLocation`)) (.z (`self.K2_GetActorLocation`))) false true)
        (if (== (.x (`self.K2_GetActorLocation`)) -250.0)
          (`self.K2_SetActorRotation` (`KismetMathLibrary.MakeRotator` 0.0 90.0))
          (`self.K2_SetActorLocation` (`KismetMathLibrary.MakeVector` (+ (.x (`self.K2_GetActorLocation`)) 49.0) (.y (`self.K2_GetActorLocation`)) (+ (.z (`self.K2_GetActorLocation`)) -51.0)) false true))))))

(fn `PositionRight`
  (bind _x (.x (`self.K2_GetActorLocation`)))
  (bind _y (.y (`self.K2_GetActorLocation`)))
  (if (== _x -201.0)
    (`self.K2_SetActorLocation` (`KismetMathLibrary.MakeVector` (.x (`self.K2_GetActorLocation`)) (+ (.y (`self.K2_GetActorLocation`)) 100.0) (.z (`self.K2_GetActorLocation`))) false true)
    (if (== (.y (`self.K2_GetActorLocation`)) 250.0)
      (`self.K2_SetActorRotation` (`KismetMathLibrary.MakeRotator` 0.0 90.0 -90.0))
      (`self.K2_SetActorLocation` (`KismetMathLibrary.MakeVector` (+ (.x (`self.K2_GetActorLocation`)) 51.0) (+ (.y (`self.K2_GetActorLocation`)) -49.0) (.z (`self.K2_GetActorLocation`))) false true))
    (elif (== _y 201.0)
      (`self.K2_SetActorLocation` (`KismetMathLibrary.MakeVector` (+ (.x (`self.K2_GetActorLocation`)) 100.0) (.y (`self.K2_GetActorLocation`)) (.z (`self.K2_GetActorLocation`))) false true)
      (if (== (.x (`self.K2_GetActorLocation`)) 250.0)
        (`self.K2_SetActorRotation` (`KismetMathLibrary.MakeRotator` 0.0 90.0 180.0))
        (`self.K2_SetActorLocation` (`KismetMathLibrary.MakeVector` (+ (.x (`self.K2_GetActorLocation`)) -49.0) (+ (.y (`self.K2_GetActorLocation`)) -51.0) (.z (`self.K2_GetActorLocation`))) false true))
      (elif (== _x 201.0)
        (`self.K2_SetActorLocation` (`KismetMathLibrary.MakeVector` (.x (`self.K2_GetActorLocation`)) (+ (.y (`self.K2_GetActorLocation`)) -100.0) (.z (`self.K2_GetActorLocation`))) false true)
        (if (== (.y (`self.K2_GetActorLocation`)) -250.0)
          (`self.K2_SetActorRotation` (`KismetMathLibrary.MakeRotator` 0.0 90.0 90.0))
          (`self.K2_SetActorLocation` (`KismetMathLibrary.MakeVector` (+ (.x (`self.K2_GetActorLocation`)) -51.0) (+ (.y (`self.K2_GetActorLocation`)) 49.0) (.z (`self.K2_GetActorLocation`))) false true))
        (elif (== _y -201.0)
          (`self.K2_SetActorLocation` (`KismetMathLibrary.MakeVector` (+ (.x (`self.K2_GetActorLocation`)) -100.0) (.y (`self.K2_GetActorLocation`)) (.z (`self.K2_GetActorLocation`))) false true)
          (if (== (.x (`self.K2_GetActorLocation`)) -250.0)
            (`self.K2_SetActorRotation` (`KismetMathLibrary.MakeRotator` 0.0 90.0))
            (`self.K2_SetActorLocation` (`KismetMathLibrary.MakeVector` (+ (.x (`self.K2_GetActorLocation`)) 49.0) (+ (.y (`self.K2_GetActorLocation`)) 51.0) (.z (`self.K2_GetActorLocation`))) false true))
          (elif (== (.z (`self.K2_GetActorLocation`)) 201.0)
            (`self.K2_SetActorLocation` (`KismetMathLibrary.MakeVector` (.x (`self.K2_GetActorLocation`)) (+ (.y (`self.K2_GetActorLocation`)) 100.0) (.z (`self.K2_GetActorLocation`))) false true)
            (if (== (.y (`self.K2_GetActorLocation`)) 250.0)
              (`self.K2_SetActorRotation` (`KismetMathLibrary.MakeRotator` 90.0))
              (`self.K2_SetActorLocation` (`KismetMathLibrary.MakeVector` (.x (`self.K2_GetActorLocation`)) (+ (.y (`self.K2_GetActorLocation`)) -49.0) (+ (.z (`self.K2_GetActorLocation`)) -51.0)) false true))
            (elif (== (.z (`self.K2_GetActorLocation`)) -201.0)
              (`self.K2_SetActorLocation` (`KismetMathLibrary.MakeVector` (.x (`self.K2_GetActorLocation`)) (+ (.y (`self.K2_GetActorLocation`)) 100.0) (.z (`self.K2_GetActorLocation`))) false true)
              (if (== (.y (`self.K2_GetActorLocation`)) 250.0)
                (`self.K2_SetActorRotation` (`KismetMathLibrary.MakeRotator` 90.0))
                (`self.K2_SetActorLocation` (`KismetMathLibrary.MakeVector` (.x (`self.K2_GetActorLocation`)) (+ (.y (`self.K2_GetActorLocation`)) -49.0) (+ (.z (`self.K2_GetActorLocation`)) 51.0)) false true)))))))))

(fn `PositionUp`
  (bind _x (.x (`self.K2_GetActorLocation`)))
  (bind _y (.y (`self.K2_GetActorLocation`)))
  (bind _x_2 (.x (`self.K2_GetActorLocation`)))
  (bind _y_2 (.y (`self.K2_GetActorLocation`)))
  (if (or (== _x_2 -201.0) (== _y_2 -201.0) (== _x_2 201.0) (== _y_2 201.0))
    (`self.K2_SetActorLocation` (`KismetMathLibrary.MakeVector` (.x (`self.K2_GetActorLocation`)) (.y (`self.K2_GetActorLocation`)) (+ (.z (`self.K2_GetActorLocation`)) 100.0)) false true)
    (if (== (.z (`self.K2_GetActorLocation`)) 250.0)
      (if (== _x -201.0)
        (`self.K2_SetActorRotation` (`KismetMathLibrary.MakeRotator` 0.0))
        (`self.K2_SetActorLocation` (`KismetMathLibrary.MakeVector` (+ (.x (`self.K2_GetActorLocation`)) 51.0) (.y (`self.K2_GetActorLocation`)) (+ (.z (`self.K2_GetActorLocation`)) -49.0)) false true)
        (elif (== _y -201.0)
          (`self.K2_SetActorRotation` (`KismetMathLibrary.MakeRotator` 0.0))
          (`self.K2_SetActorLocation` (`KismetMathLibrary.MakeVector` (.x (`self.K2_GetActorLocation`)) (+ (.y (`self.K2_GetActorLocation`)) 51.0) (+ (.z (`self.K2_GetActorLocation`)) -49.0)) false true)
          (elif (== _x 201.0)
            (`self.K2_SetActorRotation` (`KismetMathLibrary.MakeRotator` 0.0))
            (`self.K2_SetActorLocation` (`KismetMathLibrary.MakeVector` (+ (.x (`self.K2_GetActorLocation`)) -51.0) (.y (`self.K2_GetActorLocation`)) (+ (.z (`self.K2_GetActorLocation`)) -49.0)) false true)
            (elif (== _y 201.0)
              (`self.K2_SetActorRotation` (`KismetMathLibrary.MakeRotator` 0.0))
              (`self.K2_SetActorLocation` (`KismetMathLibrary.MakeVector` (.x (`self.K2_GetActorLocation`)) (+ (.y (`self.K2_GetActorLocation`)) -51.0) (+ (.z (`self.K2_GetActorLocation`)) -49.0)) false true))))))
    (elif (== (.z (`self.K2_GetActorLocation`)) 201.0)
      (`self.K2_SetActorLocation` (`KismetMathLibrary.MakeVector` (+ (.x (`self.K2_GetActorLocation`)) 100.0) (.y (`self.K2_GetActorLocation`)) (.z (`self.K2_GetActorLocation`))) false true)
      (if (== (.x (`self.K2_GetActorLocation`)) 250.0)
        (`self.K2_SetActorRotation` (`KismetMathLibrary.MakeRotator` 0.0 90.0 180.0))
        (`self.K2_SetActorLocation` (`KismetMathLibrary.MakeVector` (+ (.x (`self.K2_GetActorLocation`)) -49.0) (.y (`self.K2_GetActorLocation`)) (+ (.z (`self.K2_GetActorLocation`)) -51.0)) false true))
      (elif (== (.z (`self.K2_GetActorLocation`)) -201.0)
        (`self.K2_SetActorLocation` (`KismetMathLibrary.MakeVector` (+ (.x (`self.K2_GetActorLocation`)) -100.0) (.y (`self.K2_GetActorLocation`)) (.z (`self.K2_GetActorLocation`))) false true)
        (if (== (.x (`self.K2_GetActorLocation`)) -250.0)
          (`self.K2_SetActorRotation` (`KismetMathLibrary.MakeRotator` 0.0 90.0))
          (`self.K2_SetActorLocation` (`KismetMathLibrary.MakeVector` (+ (.x (`self.K2_GetActorLocation`)) 49.0) (.y (`self.K2_GetActorLocation`)) (+ (.z (`self.K2_GetActorLocation`)) 51.0)) false true))))))

(fn `UserConstructionScript`)
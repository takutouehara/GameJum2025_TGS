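; Large board cursor that selects one of twelve slots and rotates that part of the board, hidden while CursorMode shows the piece cursor.
; Direction functions teleport it in fixed steps, wrapping between orientations, with GameInstance flags remembering where to return from the vertical axis.
; MoveRotation matches exact location to a BP_BanmenObject RotationN call, increments MasterChecker and briefly switches W_Main images.
; ChangeColorLarge sets black or white material from MasterChecker parity.
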(event `self.ReceiveTick`
  (params (DeltaSeconds :type "Float (single-precision)"))
  ;[1 1 1] 駒カーソルが見えているなら盤面カーソルを見えなくする
  (bind _asmaster_game_instance (cast `/Game/MasterGameInstance` (`GameplayStatics.GetGameInstance`)))
  (if (`/Game/MasterGameInstance.CursorMode` _asmaster_game_instance)
    (`self.SetActorHiddenInGame` true)
    (else
      (`self.SetActorHiddenInGame` false))))

(event `self.ReceiveBeginPlay`
  ;[1 1 1] カーソルの初期配置
  (`KismetSystemLibrary.Delay` 0.1)
  (`self.K2_SetActorLocation` (0.0 150.0 200.0) false true)
  (`self.K2_SetActorRotation` (`KismetMathLibrary.MakeRotator` 0.0)))

(event `ChangeColorLarge`
  ;[1 1 1] 設置するたびにカーソルの色を変える
  (bind _asmaster_game_instance (cast `/Game/MasterGameInstance` (`GameplayStatics.GetGameInstance`)))
  (if (== (mod (`/Game/MasterGameInstance.MasterChecker` _asmaster_game_instance) 2) 0)
    (`PrimitiveComponent.SetMaterial` (`self.Plane_cursorlarge`) 0 "/Game/Material/M_CursorMaxKuro.M_CursorMaxKuro")
    (`PrimitiveComponent.SetMaterial` (`self.Plane_cursorlarge1`) 0 "/Game/Material/M_CursorMaxKuro.M_CursorMaxKuro")
    (`PrimitiveComponent.SetMaterial` (`self.Plane_cursorlarge2`) 0 "/Game/Material/M_CursorMaxKuro.M_CursorMaxKuro")
    (`PrimitiveComponent.SetMaterial` (`self.Plane_cursorlarge3`) 0 "/Game/Material/M_CursorMaxKuro.M_CursorMaxKuro")
    (else
      (`PrimitiveComponent.SetMaterial` (`self.Plane_cursorlarge`) 0 "/Game/Material/M_CursorMaxSiro.M_CursorMaxSiro")
      (`PrimitiveComponent.SetMaterial` (`self.Plane_cursorlarge1`) 0 "/Game/Material/M_CursorMaxSiro.M_CursorMaxSiro")
      (`PrimitiveComponent.SetMaterial` (`self.Plane_cursorlarge2`) 0 "/Game/Material/M_CursorMaxSiro.M_CursorMaxSiro")
      (`PrimitiveComponent.SetMaterial` (`self.Plane_cursorlarge3`) 0 "/Game/Material/M_CursorMaxSiro.M_CursorMaxSiro"))))

(event `CurSorLargeUp`
  ;[1 1 1] カーソル操作
  (`self.Position Up`))

(event `CurSorLargeLeft`
  ;[1 1 1] カーソル操作
  (`self.Position Left`))

(event `CurSorLargeDown`
  ;[1 1 1] カーソル操作
  (`self.PositionDown`))

(event `CurSorLargeRight`
  ;[1 1 1] カーソル操作
  (`self.PositionRight`))

(event `MoveRotation`
  ;[1 1 1] 盤面カーソルがある場所の盤面を回転させる
  (if (`KismetMathLibrary.EqualExactly_VectorVector` (`self.K2_GetActorLocation`) (0.0 -150.0 200.0))
    (`self.NewFunction`)
    (bind _outactors (`GameplayStatics.GetAllActorsOfClass` "/Game/Object/BP_BanmenObject.BP_BanmenObject_C"))
    (`/Game/Object/BP_BanmenObject.Rotation 1` _outactors)
    (bind _foundwidgets (`WidgetBlueprintLibrary.GetAllWidgetsOfClass` "/Game/Widget/W_Main.W_Main_C" :!label _label))
    (`/Game/Widget/W_Main.ImagesSet_M2` _foundwidgets)
    (`KismetSystemLibrary.Delay` 0.2)
    (`/Game/Widget/W_Main.ImagesSet_M1` _foundwidgets)
    (elif (`KismetMathLibrary.EqualExactly_VectorVector` (`self.K2_GetActorLocation`) (0.0 -50.0 200.0))
      (`self.NewFunction`)
      (bind _outactors_2 (`GameplayStatics.GetAllActorsOfClass` "/Game/Object/BP_BanmenObject.BP_BanmenObject_C"))
      (`/Game/Object/BP_BanmenObject.Rotation 2` _outactors_2)
      (goto _label)
      (elif (`KismetMathLibrary.EqualExactly_VectorVector` (`self.K2_GetActorLocation`) (0.0 50.0 200.0))
        (`self.NewFunction`)
        (bind _outactors_3 (`GameplayStatics.GetAllActorsOfClass` "/Game/Object/BP_BanmenObject.BP_BanmenObject_C"))
        (`/Game/Object/BP_BanmenObject.Rotation 3` _outactors_3)
        (goto _label)
        (elif (`KismetMathLibrary.EqualExactly_VectorVector` (`self.K2_GetActorLocation`) (0.0 150.0 200.0))
          (`self.NewFunction`)
          (bind _outactors_4 (`GameplayStatics.GetAllActorsOfClass` "/Game/Object/BP_BanmenObject.BP_BanmenObject_C"))
          (`/Game/Object/BP_BanmenObject.Rotation 4` _outactors_4)
          (goto _label)
          (elif (`KismetMathLibrary.EqualExactly_VectorVector` (`self.K2_GetActorLocation`) (-150.0 0.0 200.0))
            (`self.NewFunction`)
            (bind _outactors_5 (`GameplayStatics.GetAllActorsOfClass` "/Game/Object/BP_BanmenObject.BP_BanmenObject_C"))
            (`/Game/Object/BP_BanmenObject.Rotation 5` _outactors_5)
            (goto _label)
            (elif (`KismetMathLibrary.EqualExactly_VectorVector` (`self.K2_GetActorLocation`) (-50.0 0.0 200.0))
              (`self.NewFunction`)
              (bind _outactors_6 (`GameplayStatics.GetAllActorsOfClass` "/Game/Object/BP_BanmenObject.BP_BanmenObject_C"))
              (`/Game/Object/BP_BanmenObject.Rotation 6` _outactors_6)
              (goto _label)
              (elif (`KismetMathLibrary.EqualExactly_VectorVector` (`self.K2_GetActorLocation`) (50.0 0.0 200.0))
                (`self.NewFunction`)
                (bind _outactors_7 (`GameplayStatics.GetAllActorsOfClass` "/Game/Object/BP_BanmenObject.BP_BanmenObject_C"))
                (`/Game/Object/BP_BanmenObject.Rotation 7` _outactors_7)
                (goto _label)
                (elif (`KismetMathLibrary.EqualExactly_VectorVector` (`self.K2_GetActorLocation`) (150.0 0.0 200.0))
                  (`self.NewFunction`)
                  (bind _outactors_8 (`GameplayStatics.GetAllActorsOfClass` "/Game/Object/BP_BanmenObject.BP_BanmenObject_C"))
                  (`/Game/Object/BP_BanmenObject.Rotation 8` _outactors_8)
                  (goto _label)
                  (elif (`KismetMathLibrary.EqualExactly_VectorVector` (`self.K2_GetActorLocation`) (0.0 200.0 -150.0))
                    (`self.NewFunction`)
                    (bind _outactors_9 (`GameplayStatics.GetAllActorsOfClass` "/Game/Object/BP_BanmenObject.BP_BanmenObject_C"))
                    (`/Game/Object/BP_BanmenObject.Rotation 9` _outactors_9)
                    (goto _label)
                    (elif (`KismetMathLibrary.EqualExactly_VectorVector` (`self.K2_GetActorLocation`) (0.0 200.0 -50.0))
                      (`self.NewFunction`)
                      (bind _outactors_10 (`GameplayStatics.GetAllActorsOfClass` "/Game/Object/BP_BanmenObject.BP_BanmenObject_C"))
                      (`/Game/Object/BP_BanmenObject.Rotation 10` _outactors_10)
                      (goto _label)
                      (elif (`KismetMathLibrary.EqualExactly_VectorVector` (`self.K2_GetActorLocation`) (0.0 200.0 50.0))
                        (`self.NewFunction`)
                        (bind _outactors_11 (`GameplayStatics.GetAllActorsOfClass` "/Game/Object/BP_BanmenObject.BP_BanmenObject_C"))
                        (`/Game/Object/BP_BanmenObject.Rotation 11` _outactors_11)
                        (goto _label)
                        (elif (`KismetMathLibrary.EqualExactly_VectorVector` (`self.K2_GetActorLocation`) (0.0 200.0 150.0))
                          (`self.NewFunction`)
                          (bind _outactors_12 (`GameplayStatics.GetAllActorsOfClass` "/Game/Object/BP_BanmenObject.BP_BanmenObject_C"))
                          (`/Game/Object/BP_BanmenObject.Rotation 12` _outactors_12)
                          (goto _label))))))))))))))

(fn `NewFunction`
  (bind _asmaster_game_instance (cast `/Game/MasterGameInstance` (`GameplayStatics.GetGameInstance`)))
  (bind _result (`/Engine/EditorBlueprintResources/StandardMacros.IncrementInt` (`/Game/MasterGameInstance.MasterChecker` _asmaster_game_instance))
    (:`  `
      (set `/Game/MasterGameInstance.MasterChecker` _result _asmaster_game_instance))))

(fn `Position Left`
  (bind _yaw (.yaw (`self.K2_GetActorRotation`)))
  (if (and (`KismetMathLibrary.NearlyEqual_FloatFloat` _yaw 0.0 0.001) (`KismetMathLibrary.NearlyEqual_FloatFloat` (.roll (`self.K2_GetActorRotation`)) 0.0 0.001))
    (`self.K2_SetActorLocation` (`KismetMathLibrary.MakeVector` (.x (`self.K2_GetActorLocation`)) (+ (.y (`self.K2_GetActorLocation`)) -100.0) (.z (`self.K2_GetActorLocation`))) false true)
    (if (== (.y (`self.K2_GetActorLocation`)) -250.0)
      (`self.K2_SetActorRotation` (`KismetMathLibrary.MakeRotator` 0.0 0.0 90.0))
      (`self.K2_SetActorLocation` (-150.0 0.0 200.0) false true))
    (elif (`KismetMathLibrary.NearlyEqual_FloatFloat` _yaw 90.0 0.001)
      (`self.K2_SetActorLocation` (`KismetMathLibrary.MakeVector` (+ (.x (`self.K2_GetActorLocation`)) 100.0) (.y (`self.K2_GetActorLocation`)) (.z (`self.K2_GetActorLocation`))) false true)
      (if (== (.x (`self.K2_GetActorLocation`)) 250.0)
        (`self.K2_SetActorRotation` (`KismetMathLibrary.MakeRotator` 0.0 0.0 180.0))
        (`self.K2_SetActorLocation` (0.0 -150.0 200.0) false true))
      (elif (`KismetMathLibrary.NearlyEqual_FloatFloat` _yaw 180.0 0.001)
        (`self.K2_SetActorLocation` (`KismetMathLibrary.MakeVector` (.x (`self.K2_GetActorLocation`)) (+ (.y (`self.K2_GetActorLocation`)) 100.0) (.z (`self.K2_GetActorLocation`))) false true)
        (if (== (.y (`self.K2_GetActorLocation`)) 250.0)
          (`self.K2_SetActorRotation` (`KismetMathLibrary.MakeRotator` 0.0 0.0 -90.0))
          (`self.K2_SetActorLocation` (150.0 0.0 200.0) false true))
        (elif (`KismetMathLibrary.NearlyEqual_FloatFloat` _yaw -90.0 0.001)
          (`self.K2_SetActorLocation` (`KismetMathLibrary.MakeVector` (+ (.x (`self.K2_GetActorLocation`)) -100.0) (.y (`self.K2_GetActorLocation`)) (.z (`self.K2_GetActorLocation`))) false true)
          (if (== (.x (`self.K2_GetActorLocation`)) -250.0)
            (`self.K2_SetActorRotation` (`KismetMathLibrary.MakeRotator` 0.0))
            (`self.K2_SetActorLocation` (0.0 150.0 200.0) false true)))))))

(fn `Position Up`
  (if (`KismetMathLibrary.NearlyEqual_FloatFloat` (.roll (`self.K2_GetActorRotation`)) 90.0 0.001)
    (`self.K2_SetActorLocation` (`KismetMathLibrary.MakeVector` (.x (`self.K2_GetActorLocation`)) (.y (`self.K2_GetActorLocation`)) (+ (.z (`self.K2_GetActorLocation`)) 100.0)) false true)
    (if (== (.z (`self.K2_GetActorLocation`)) 250.0)
      (bind _asmaster_game_instance (cast `/Game/MasterGameInstance` (`GameplayStatics.GetGameInstance`)))
      (if (`/Game/MasterGameInstance.FrontMove` _asmaster_game_instance)
        (`self.K2_SetActorRotation` (`KismetMathLibrary.MakeRotator` 0.0))
        (`self.K2_SetActorLocation` (0.0 50.0 200.0) false true)
        (elif (`/Game/MasterGameInstance.LeftMove` _asmaster_game_instance)
          (`self.K2_SetActorRotation` (`KismetMathLibrary.MakeRotator` 0.0 0.0 90.0))
          (`self.K2_SetActorLocation` (-50.0 0.0 200.0) false true)
          (elif (`/Game/MasterGameInstance.BackMove` _asmaster_game_instance)
            (`self.K2_SetActorRotation` (`KismetMathLibrary.MakeRotator` 0.0 0.0 180.0))
            (`self.K2_SetActorLocation` (0.0 -50.0 200.0) false true)
            (elif (`/Game/MasterGameInstance.RightMove` _asmaster_game_instance)
              (`self.K2_SetActorRotation` (`KismetMathLibrary.MakeRotator` 0.0 0.0 -90.0))
              (`self.K2_SetActorLocation` (50.0 0.0 200.0) false true))))))
    (elif (`KismetMathLibrary.NearlyEqual_FloatFloat` (.yaw (`self.K2_GetActorRotation`)) 0.0 0.001)
      (`self.K2_SetActorRotation` (`KismetMathLibrary.MakeRotator` 90.0))
      (`self.K2_SetActorLocation` (0.0 200.0 150.0) false true)
      (bind _asmaster_game_instance_2 (cast `/Game/MasterGameInstance` (`GameplayStatics.GetGameInstance`)))
      (set `/Game/MasterGameInstance.FrontMove` true _asmaster_game_instance_2)
      (set `/Game/MasterGameInstance.LeftMove` false _asmaster_game_instance_2)
      (set `/Game/MasterGameInstance.BackMove` false _asmaster_game_instance_2)
      (set `/Game/MasterGameInstance.RightMove` false _asmaster_game_instance_2)
      (elif (`KismetMathLibrary.NearlyEqual_FloatFloat` (.yaw (`self.K2_GetActorRotation`)) 90.0 0.001)
        (`self.K2_SetActorRotation` (`KismetMathLibrary.MakeRotator` 90.0))
        (`self.K2_SetActorLocation` (0.0 200.0 150.0) false true)
        (bind _asmaster_game_instance_3 (cast `/Game/MasterGameInstance` (`GameplayStatics.GetGameInstance`)))
        (set `/Game/MasterGameInstance.FrontMove` false _asmaster_game_instance_3)
        (set `/Game/MasterGameInstance.LeftMove` true _asmaster_game_instance_3)
        (set `/Game/MasterGameInstance.BackMove` false _asmaster_game_instance_3)
        (set `/Game/MasterGameInstance.RightMove` false _asmaster_game_instance_3)
        (elif (`KismetMathLibrary.NearlyEqual_FloatFloat` (.yaw (`self.K2_GetActorRotation`)) 180.0 0.001)
          (`self.K2_SetActorRotation` (`KismetMathLibrary.MakeRotator` 90.0))
          (`self.K2_SetActorLocation` (0.0 200.0 150.0) false true)
          (bind _asmaster_game_instance_4 (cast `/Game/MasterGameInstance` (`GameplayStatics.GetGameInstance`)))
          (set `/Game/MasterGameInstance.FrontMove` false _asmaster_game_instance_4)
          (set `/Game/MasterGameInstance.LeftMove` false _asmaster_game_instance_4)
          (set `/Game/MasterGameInstance.BackMove` true _asmaster_game_instance_4)
          (set `/Game/MasterGameInstance.RightMove` false _asmaster_game_instance_4)
          (elif (`KismetMathLibrary.NearlyEqual_FloatFloat` (.yaw (`self.K2_GetActorRotation`)) -90.0 0.001)
            (`self.K2_SetActorRotation` (`KismetMathLibrary.MakeRotator` 90.0))
            (`self.K2_SetActorLocation` (0.0 200.0 150.0) false true)
            (bind _asmaster_game_instance_5 (cast `/Game/MasterGameInstance` (`GameplayStatics.GetGameInstance`)))
            (set `/Game/MasterGameInstance.FrontMove` false _asmaster_game_instance_5)
            (set `/Game/MasterGameInstance.LeftMove` false _asmaster_game_instance_5)
            (set `/Game/MasterGameInstance.BackMove` false _asmaster_game_instance_5)
            (set `/Game/MasterGameInstance.RightMove` true _asmaster_game_instance_5)))))))

(fn `PositionDown`
  (if (`KismetMathLibrary.NearlyEqual_FloatFloat` (.roll (`self.K2_GetActorRotation`)) 90.0 0.001)
    (`self.K2_SetActorLocation` (`KismetMathLibrary.MakeVector` (.x (`self.K2_GetActorLocation`)) (.y (`self.K2_GetActorLocation`)) (+ (.z (`self.K2_GetActorLocation`)) -100.0)) false true)
    (if (== (.z (`self.K2_GetActorLocation`)) -250.0)
      (bind _asmaster_game_instance (cast `/Game/MasterGameInstance` (`GameplayStatics.GetGameInstance`)))
      (if (`/Game/MasterGameInstance.FrontMove` _asmaster_game_instance)
        (`self.K2_SetActorRotation` (`KismetMathLibrary.MakeRotator` 0.0))
        (`self.K2_SetActorLocation` (0.0 50.0 200.0) false true)
        (elif (`/Game/MasterGameInstance.LeftMove` _asmaster_game_instance)
          (`self.K2_SetActorRotation` (`KismetMathLibrary.MakeRotator` 0.0 0.0 90.0))
          (`self.K2_SetActorLocation` (-50.0 0.0 200.0) false true)
          (elif (`/Game/MasterGameInstance.BackMove` _asmaster_game_instance)
            (`self.K2_SetActorRotation` (`KismetMathLibrary.MakeRotator` 0.0 0.0 180.0))
            (`self.K2_SetActorLocation` (0.0 -50.0 200.0) false true)
            (elif (`/Game/MasterGameInstance.RightMove` _asmaster_game_instance)
              (`self.K2_SetActorRotation` (`KismetMathLibrary.MakeRotator` 0.0 0.0 -90.0))
              (`self.K2_SetActorLocation` (50.0 0.0 200.0) false true))))))
    (elif (`KismetMathLibrary.NearlyEqual_FloatFloat` (.yaw (`self.K2_GetActorRotation`)) 0.0 0.001)
      (`self.K2_SetActorRotation` (`KismetMathLibrary.MakeRotator` 90.0))
      (`self.K2_SetActorLocation` (0.0 200.0 -150.0) false true)
      (bind _asmaster_game_instance_2 (cast `/Game/MasterGameInstance` (`GameplayStatics.GetGameInstance`)))
      (set `/Game/MasterGameInstance.FrontMove` true _asmaster_game_instance_2)
      (set `/Game/MasterGameInstance.LeftMove` false _asmaster_game_instance_2)
      (set `/Game/MasterGameInstance.BackMove` false _asmaster_game_instance_2)
      (set `/Game/MasterGameInstance.RightMove` false _asmaster_game_instance_2)
      (elif (`KismetMathLibrary.NearlyEqual_FloatFloat` (.yaw (`self.K2_GetActorRotation`)) 90.0 0.001)
        (`self.K2_SetActorRotation` (`KismetMathLibrary.MakeRotator` 90.0))
        (`self.K2_SetActorLocation` (0.0 200.0 -150.0) false true)
        (bind _asmaster_game_instance_3 (cast `/Game/MasterGameInstance` (`GameplayStatics.GetGameInstance`)))
        (set `/Game/MasterGameInstance.FrontMove` false _asmaster_game_instance_3)
        (set `/Game/MasterGameInstance.LeftMove` true _asmaster_game_instance_3)
        (set `/Game/MasterGameInstance.BackMove` false _asmaster_game_instance_3)
        (set `/Game/MasterGameInstance.RightMove` false _asmaster_game_instance_3)
        (elif (`KismetMathLibrary.NearlyEqual_FloatFloat` (.yaw (`self.K2_GetActorRotation`)) 180.0 0.001)
          (`self.K2_SetActorRotation` (`KismetMathLibrary.MakeRotator` 90.0))
          (`self.K2_SetActorLocation` (0.0 200.0 -150.0) false true)
          (bind _asmaster_game_instance_4 (cast `/Game/MasterGameInstance` (`GameplayStatics.GetGameInstance`)))
          (set `/Game/MasterGameInstance.FrontMove` false _asmaster_game_instance_4)
          (set `/Game/MasterGameInstance.LeftMove` false _asmaster_game_instance_4)
          (set `/Game/MasterGameInstance.BackMove` true _asmaster_game_instance_4)
          (set `/Game/MasterGameInstance.RightMove` false _asmaster_game_instance_4)
          (elif (`KismetMathLibrary.NearlyEqual_FloatFloat` (.yaw (`self.K2_GetActorRotation`)) -90.0 0.001)
            (`self.K2_SetActorRotation` (`KismetMathLibrary.MakeRotator` 90.0))
            (`self.K2_SetActorLocation` (0.0 200.0 -150.0) false true)
            (bind _asmaster_game_instance_5 (cast `/Game/MasterGameInstance` (`GameplayStatics.GetGameInstance`)))
            (set `/Game/MasterGameInstance.FrontMove` false _asmaster_game_instance_5)
            (set `/Game/MasterGameInstance.LeftMove` false _asmaster_game_instance_5)
            (set `/Game/MasterGameInstance.BackMove` false _asmaster_game_instance_5)
            (set `/Game/MasterGameInstance.RightMove` true _asmaster_game_instance_5)))))))

(fn `PositionRight`
  (bind _yaw (.yaw (`self.K2_GetActorRotation`)))
  (if (and (`KismetMathLibrary.NearlyEqual_FloatFloat` _yaw 0.0 0.001) (`KismetMathLibrary.NearlyEqual_FloatFloat` (.roll (`self.K2_GetActorRotation`)) 0.0 0.001))
    (`self.K2_SetActorLocation` (`KismetMathLibrary.MakeVector` (.x (`self.K2_GetActorLocation`)) (+ (.y (`self.K2_GetActorLocation`)) 100.0) (.z (`self.K2_GetActorLocation`))) false true)
    (if (== (.y (`self.K2_GetActorLocation`)) 250.0)
      (`self.K2_SetActorRotation` (`KismetMathLibrary.MakeRotator` 0.0 0.0 -90.0))
      (`self.K2_SetActorLocation` (-150.0 0.0 200.0) false true))
    (elif (`KismetMathLibrary.NearlyEqual_FloatFloat` _yaw -90.0 0.001)
      (`self.K2_SetActorLocation` (`KismetMathLibrary.MakeVector` (+ (.x (`self.K2_GetActorLocation`)) 100.0) (.y (`self.K2_GetActorLocation`)) (.z (`self.K2_GetActorLocation`))) false true)
      (if (== (.x (`self.K2_GetActorLocation`)) 250.0)
        (`self.K2_SetActorRotation` (`KismetMathLibrary.MakeRotator` 0.0 0.0 180.0))
        (`self.K2_SetActorLocation` (0.0 150.0 200.0) false true))
      (elif (`KismetMathLibrary.NearlyEqual_FloatFloat` _yaw 180.0 0.001)
        (`self.K2_SetActorLocation` (`KismetMathLibrary.MakeVector` (.x (`self.K2_GetActorLocation`)) (+ (.y (`self.K2_GetActorLocation`)) -100.0) (.z (`self.K2_GetActorLocation`))) false true)
        (if (== (.y (`self.K2_GetActorLocation`)) -250.0)
          (`self.K2_SetActorRotation` (`KismetMathLibrary.MakeRotator` 0.0 0.0 90.0))
          (`self.K2_SetActorLocation` (150.0 0.0 200.0) false true))
        (elif (`KismetMathLibrary.NearlyEqual_FloatFloat` _yaw 90.0 0.001)
          (`self.K2_SetActorLocation` (`KismetMathLibrary.MakeVector` (+ (.x (`self.K2_GetActorLocation`)) -100.0) (.y (`self.K2_GetActorLocation`)) (.z (`self.K2_GetActorLocation`))) false true)
          (if (== (.x (`self.K2_GetActorLocation`)) -250.0)
            (`self.K2_SetActorRotation` (`KismetMathLibrary.MakeRotator` 0.0))
            (`self.K2_SetActorLocation` (0.0 -150.0 200.0) false true)))))))

(fn `UserConstructionScript`)
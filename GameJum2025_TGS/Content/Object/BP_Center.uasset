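; BP_Center is an actor that turns itself in a short stepped rotation when its TestTest event fires.
; The event sets a flag that Tick polls, using a Delay to space out fixed 10-degree local rotation increments.
; A counter ends the turn after nine steps, about 90 degrees, then resets along with the flag.
; Each step prints the actor's pitch as debug output.
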(event `TestTest`
  (set `self.NewVar_0` true))

(event `self.ReceiveTick`
  (params (DeltaSeconds :type "Float (single-precision)"))
  (if (`self.NewVar_0`)
    (if (< (`self.NewVar`) 9)
      (`KismetSystemLibrary.Delay` 0.1)
      (bind _result (`/Engine/EditorBlueprintResources/StandardMacros.IncrementInt` (`self.NewVar`))
        (:`  `
          (set `self.NewVar` _result)
          (`self.K2_AddActorLocalRotation` (struct :`Pitch` 10.0))
          (`KismetSystemLibrary.PrintString` (`KismetStringLibrary.Conv_DoubleToString` (.pitch (`self.K2_GetActorRotation`))))))
      (else
        (set `self.NewVar_0` false)
        (set `self.NewVar` 0)))))

(fn `UserConstructionScript`)
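; BP_BanmenObject is a board piece that makes layer-style quarter turns around BP_Center, similar to a twisty cube puzzle.
; Debug01–03 flag the piece when its Y, X or Z position matches that axis's outer plane.
; Tick then applies delay-paced 10-degree steps, orbiting its location and adding local rotation until a shared counter reaches nine.
; The twelve Rotation events and Debug04 are empty.
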(event `Rotation 1`
  ;[1 1 1] コメント
)

(event `Rotation 5`
  ;[1 1 1] コメント
)

(event `Rotation 9`
  ;[1 1 1] コメント
)

(event `Debug01`
  (if (`KismetMathLibrary.NearlyEqual_FloatFloat` (.y (`self.K2_GetActorLocation`)) -150.0 0.001)
    (set `self.Checker Y-150` true)))

(event `Debug02`
  (if (`KismetMathLibrary.NearlyEqual_FloatFloat` (.x (`self.K2_GetActorLocation`)) -150.0 0.001)
    (set `self.Checker X-150` true)))

(event `Debug03`
  (if (`KismetMathLibrary.NearlyEqual_FloatFloat` (.z (`self.K2_GetActorLocation`)) 150.0 0.001)
    (set `self.Checker Z150` true)))

(event `Rotation 2`
  ;[1 1 1] コメント
)

(event `Rotation 6`
  ;[1 1 1] コメント
)

(event `Rotation 10`
  ;[1 1 1] コメント
)

(event `Rotation 3`
  ;[1 1 1] コメント
)

(event `Rotation 7`
  ;[1 1 1] コメント
)

(event `Rotation 11`
  ;[1 1 1] コメント
)

(event `Rotation 4`
  ;[1 1 1] コメント
)

(event `Rotation 8`
  ;[1 1 1] コメント
)

(event `Rotation 12`
  ;[1 1 1] コメント
)

(event `Debug04`)

(event `self.ReceiveTick`
  (params (DeltaSeconds :type "Float (single-precision)"))
  (`|ExecutionSequence`
    (:`then_1`
      (if (`self.Checker Y-150`)
        (if (< (`self.RowlingCounter`) 9)
          (bind _returnvalue (`GameplayStatics.GetActorOfClass` "/Game/Object/BP_Center.BP_Center_C"))
          (`KismetSystemLibrary.Delay` 0.1)
          (bind _result (`/Engine/EditorBlueprintResources/StandardMacros.IncrementInt` (`self.RowlingCounter`))
            (:`  `
              (set `self.RowlingCounter` _result)
              (bind _returnvalue_2 (`self.K2_GetActorLocation` _returnvalue))
              (`self.K2_SetActorLocation` (+ (`KismetMathLibrary.GreaterGreater_VectorRotator` (- (`self.K2_GetActorLocation`) _returnvalue_2) (struct :`Pitch` 10.0)) _returnvalue_2) false true)
              (`self.K2_AddActorLocalRotation` (struct :`Pitch` 10.0))))
          (else
            (set `self.Checker Y-150` false)
            (set `self.RowlingCounter` 0)))))
    (:`then_2`
      (if (`self.Checker X-150`)
        (if (< (`self.RowlingCounter`) 9)
          (bind _returnvalue_3 (`GameplayStatics.GetActorOfClass` "/Game/Object/BP_Center.BP_Center_C"))
          (`KismetSystemLibrary.Delay` 0.1)
          (bind _result_2 (`/Engine/EditorBlueprintResources/StandardMacros.IncrementInt` (`self.RowlingCounter`))
            (:`  `
              (set `self.RowlingCounter` _result_2)
              (bind _returnvalue_4 (`self.K2_GetActorLocation` _returnvalue_3))
              (`self.K2_SetActorLocation` (+ (`KismetMathLibrary.GreaterGreater_VectorRotator` (- (`self.K2_GetActorLocation`) _returnvalue_4) (struct :`Roll` 10.0)) _returnvalue_4) false true)
              (`self.K2_AddActorLocalRotation` (struct :`Roll` 10.0))))
          (else
            (set `self.Checker X-150` false)
            (set `self.RowlingCounter` 0)))))
    (:`then_3`
      (if (`self.Checker Z150`)
        (if (< (`self.RowlingCounter`) 9)
          (bind _returnvalue_5 (`GameplayStatics.GetActorOfClass` "/Game/Object/BP_Center.BP_Center_C"))
          (`KismetSystemLibrary.Delay` 0.1)
          (bind _result_3 (`/Engine/EditorBlueprintResources/StandardMacros.IncrementInt` (`self.RowlingCounter`))
            (:`  `
              (set `self.RowlingCounter` _result_3)
              (bind _returnvalue_6 (`self.K2_GetActorLocation` _returnvalue_5))
              (`self.K2_SetActorLocation` (+ (`KismetMathLibrary.GreaterGreater_VectorRotator` (- (`self.K2_GetActorLocation`) _returnvalue_6) (struct :`Yaw` 10.0)) _returnvalue_6) false true)
              (`self.K2_AddActorLocalRotation` (struct :`Yaw` 10.0))))
          (else
            (set `self.Checker Z150` false)
            (set `self.RowlingCounter` 0)))))))

(fn `UserConstructionScript`)
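; BP_Shoulderbutton is a Blueprint that switches the view between its two cameras, Camera and Camera1, with the gamepad shoulder buttons.
; The SwitchCameraLeft (LB) and SwitchCameraRight (RB) input action events each check whether Camera is active, then deactivate one camera and activate the other.
; Both events run identical toggle logic, so either button flips to the other camera regardless of direction.
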(event `InputAction|SwitchCameraLeft`
  (params (Key :type "Key Structure"))
  ;[1 1 1] 左LBキー
  (:`Pressed`
    (if (`ActorComponent.IsActive` (`self.Camera`))
      (`ActorComponent.Deactivate` (`self.Camera`))
      (`ActorComponent.SetActive` (`self.Camera1`) true false)
      (else
        (`ActorComponent.Deactivate` (`self.Camera1`))
        (`ActorComponent.SetActive` (`self.Camera`) true false)))))

(event `InputAction|SwitchCameraRight`
  (params (Key :type "Key Structure"))
  ;[1 1 1] 右RBキー
  (:`Pressed`
    (if (`ActorComponent.IsActive` (`self.Camera`))
      (`ActorComponent.Deactivate` (`self.Camera`))
      (`ActorComponent.SetActive` (`self.Camera1`) true false)
      (else
        (`ActorComponent.Deactivate` (`self.Camera1`))
        (`ActorComponent.SetActive` (`self.Camera`) true false)))))

(fn `UserConstructionScript`)